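; BP_PV_Shooter is a shooter game-flow Blueprint that handles the start menu and team scoring.
; BeginPlay adds the shooter UI and a play-menu widget to the viewport, then pauses the game until Play_game removes the menu and unpauses.
; IncrementTeamScore increments a team's entry in the TeamScores map, keyed by team byte, and calls ScoreUpdated with that team.
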(event Custom|Play_game
  (Widget|RemovefromParent (Variables|Default|GetPauseMenu))
  (Game|SetGamePaused false))

(event EventBeginPlay
  ;[0.15 0.15 0.15 0.5] Game initialization with a play interface
  (bind _returnvalue (UserInterface|CreateWidget "/Game/Variant_Shooter/UI/UI_Shooter.UI_Shooter_C"))
  (UserInterface|Viewport|AddtoViewport _returnvalue 0)
  (bind _returnvalue_2 (UserInterface|CreateWidget "/Game/DEV_G03_P3/UI/PV_PlayWidgetBlueprint.PV_PlayWidgetBlueprint_C"))
  (Variables|Default|SetPauseMenu _returnvalue_2)
  (UserInterface|Viewport|AddtoViewport _returnvalue_2 0)
  (Game|SetGamePaused true))

(event EventIncrementTeamScore
  (params (TeamByte :type Byte :default 0))
  (bind _teamscores (Variables|Default|GetTeamScores))
  (Utilities|Map|Add _teamscores TeamByte (+ (.Value (Utilities|Map|Find _teamscores TeamByte)) 1))
  (Default|CallScoreUpdated TeamByte))

(fn ConstructionScript)