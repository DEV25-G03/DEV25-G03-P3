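; PV_Shooter handles game start and team score tracking for what its name indicates is a shooter.
; On BeginPlay it shows a play-menu widget and pauses the game until the Play_game event removes the menu and unpauses.
; Scores live in a map keyed by team byte; IncrementTeamScore adds one and fires a ScoreUpdated dispatcher, while GetTeamScore returns a team's current value.
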(event Custom|Play_game
  (Widget|RemovefromParent (Variables|Default|GetPlayMenu))
  (Game|SetGamePaused false))

(event EventBeginPlay
  ;[0.15 0.15 0.15 0.5] Game initialization with a play interface
  (bind _returnvalue (UserInterface|CreateWidget "/Game/DEV_G03_P3/UI/PV_PlayWidgetBlueprint.PV_PlayWidgetBlueprint_C"))
  (Variables|Default|SetPlayMenu _returnvalue)
  (UserInterface|Viewport|AddtoViewport _returnvalue 0)
  (Game|SetGamePaused true))

(event EventIncrementTeamScore
  (params (TeamByte :type Byte :default 0))
  (bind _teamscores (Variables|Default|GetTeamScores))
  (Utilities|Map|Add _teamscores TeamByte (+ (.Value (Utilities|Map|Find _teamscores TeamByte)) 1))
  (Default|CallScoreUpdated TeamByte))

(fn ConstructionScript)

(fn GetTeamScore
  (params (NewParam :type Byte :default 0))
  (return NewParam (.Value (Utilities|Map|Find (Variables|Default|GetTeamScores) NewParam))))